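; Master enemy Blueprint that roams at random and registers itself on the player's compass.
; A looping AI MoveTo picks reachable points within a radius and pauses for a random delay after each successful move.
; A sphere overlap, or an initialization check, adds the enemy through a component on the overlapping actor, and leaving the sphere removes it.
; While it moves on the compass, a looping timer updates the HUD, and stopping clears the timer.
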(event `self.ReceiveBeginPlay`
  ;[0.05098 0.05098 0.05098] Begin Play
  (`KismetSystemLibrary.Delay` 0.01)
  (`self.RandomRoam`))

(event `RandomRoam`
  ;[0.05098 0.05098 0.05098] Random Roam Logic
  (`self.OnStartMoving`)
  (`|AIMoveTo` self (`NavigationSystemV1.K2_GetRandomReachablePointInRadius` (`self.K2_GetActorLocation`) (`self.MoveRadius`) null null) null
    (:`OnSuccess`
      (`self.OnStopMoving`)
      (`KismetSystemLibrary.Delay` (`KismetMathLibrary.RandomFloatInRange` (`self.MinDelayDuration`) (`self.MaxDelayDuration`)))
      (`self.RandomRoam`))))

(event `StartUpdateTimer`
  ;[0.05098 0.05098 0.05098] Creates the Timer That Tells the Player's Compass How Often It Should Update the Enemy's Position and Distance
  (bind _returnvalue (`KismetSystemLibrary.K2_SetTimerDelegate` (delegate `UpdateOnCompass`) (`self.CompassUpdateInterval`) true))
  (set `self.UpdateCompassTimer` _returnvalue))

(event `UpdateOnCompass`
  ;[0.05098 0.05098 0.05098] Creates the Timer That Tells the Player's Compass How Often It Should Update the Enemy's Position and Distance
  (`self.OnEnemyMove` (`.PlayerHUDRef` (`self.PlayerHUDRef`)) self))

(event `self.OnCompassSphere.OnComponentBeginOverlap`
  (params (OverlappedComponent :type "PrimitiveComponent Object Reference") (OtherActor :type "Actor Object Reference") (OtherComp :type "PrimitiveComponent Object Reference") (OtherBodyIndex :type Integer) (bFromSweep :type Boolean) (SweepResult :type "HitResult Structure (by ref)"))
  (bind _returnvalue (`self.GetComponentByClass` OtherActor null))
  ;[0.05098 0.05098 0.05098] Add the Enemy to the Player's Compass When the Player is Inside the OnCompassSphere Collider
  (if (not (`self.isOnCompass`))
    (`/Engine/EditorBlueprintResources/StandardMacros.IsValid` _returnvalue
      (:`Is Valid`
        (bind _issuccess (`self.AddEnemyToCompass` _returnvalue self))
        (if _issuccess
          (set `self.isOnCompass` true)
          (set `self.PlayerHUDRef` null _returnvalue)
          (if (`self.isMoving`)
            (`self.StartUpdateTimer`)))))))

(event `self.OnCompassSphere.OnComponentEndOverlap`
  (params (OverlappedComponent :type "PrimitiveComponent Object Reference") (OtherActor :type "Actor Object Reference") (OtherComp :type "PrimitiveComponent Object Reference") (OtherBodyIndex :type Integer))
  (bind _returnvalue (`self.GetComponentByClass` OtherActor null))
  ;[0.05098 0.05098 0.05098] Remove the Enemy from the Player's Compass When the Player Leaves the OnCompassSphere Collider
  (if (`self.isOnCompass`)
    (`/Engine/EditorBlueprintResources/StandardMacros.IsValid` _returnvalue
      (:`Is Valid`
        (set `self.isOnCompass` false)
        (`KismetSystemLibrary.K2_ClearAndInvalidateTimerHandle` (`self.UpdateCompassTimer`))
        (`self.RemoveEnemyFromCompass` _returnvalue self)
        (set `self.PlayerHUDRef` null)))))

(event `OnStartMoving`
  ;[0.05098 0.05098 0.05098] When the Enemy Moves
  (set `self.isMoving` true)
  (if (`self.isOnCompass`)
    (`/Engine/EditorBlueprintResources/StandardMacros.IsValid` (`.PlayerHUDRef` (`self.PlayerHUDRef`))
      (:`Is Valid`
        (`self.UpdateOnCompass`)
        (`self.StartUpdateTimer`))
      (:`Is Not Valid`
        (`KismetSystemLibrary.PrintString` "ERROR: Compass Widget Reference Not Valid in Main Enemy Blueprint" true true (struct :`R` 1.0 :`A` 1.0) 5.0)))))

(event `OnStopMoving`
  ;[0.05098 0.05098 0.05098] Whe nthe Enemy Stops moving
  (set `self.isMoving` false)
  (`KismetSystemLibrary.K2_ClearAndInvalidateTimerHandle` (`self.UpdateCompassTimer`))
  (if (`self.isOnCompass`)
    (`/Engine/EditorBlueprintResources/StandardMacros.IsValid` (`.PlayerHUDRef` (`self.PlayerHUDRef`))
      (:`Is Valid`
        (`self.UpdateOnCompass`))
      (:`Is Not Valid`
        (`KismetSystemLibrary.PrintString` "ERROR: Compass Widget Reference Not Valid in Main Enemy Blueprint" true true (struct :`R` 1.0 :`A` 1.0) 5.0)))))

(event `OnCompassInitialize`
  ;[0.05098 0.05098 0.05098] To Be Called When the Game Starts. If an Enemy Should be on the Compass, it will be Added on
  (for _array_element (`PrimitiveComponent.GetOverlappingActors` (`self.OnCompassSphere`) "/Script/Engine.Character")
    (bind _returnvalue (`self.GetComponentByClass` _array_element null))
    (`/Engine/EditorBlueprintResources/StandardMacros.IsValid` _returnvalue
      (:`Is Valid`
        (bind _issuccess (`self.AddEnemyToCompass` _returnvalue self))
        (if _issuccess
          (set `self.isOnCompass` true)
          (set `self.PlayerHUDRef` null _returnvalue)
          (break))))))

(fn `UserConstructionScript`
  (set `self.MoveRadius` (`self.MoveRadius`))
  (set `self.MinDelayDuration` (`self.MinDelayDuration`))
  (set `self.MaxDelayDuration` (`self.MaxDelayDuration`))
  (set `CharacterMovementComponent.MaxWalkSpeed` (`self.MovementSpeed`) (`self.CharacterMovement`))
  (`SphereComponent.SetSphereRadius` (`self.OnCompassSphere`) (`self.OnCompassRadius`) false))