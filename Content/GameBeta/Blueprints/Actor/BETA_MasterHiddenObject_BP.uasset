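; Master Blueprint actor for hidden objects that notifies the player HUD when something enters or leaves its highlight range.
; The construction script sizes the HighlightRange sphere from the HighlightRadius variable.
; On overlap begin and end, it looks up the main HUD component on the other actor and, if found, passes itself to that component's enter or leave range handler.
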(event `self.HighlightRange.OnComponentBeginOverlap`
  (params (OverlappedComponent :type "PrimitiveComponent Object Reference") (OtherActor :type "Actor Object Reference") (OtherComp :type "PrimitiveComponent Object Reference") (OtherBodyIndex :type Integer) (bFromSweep :type Boolean) (SweepResult :type "HitResult Structure (by ref)"))
  (bind _returnvalue (`self.GetComponentByClass` OtherActor "/Game/Game/Blueprints/Component/Actor/BETA_MainHUDComponent_BPC.BETA_MainHUDComponent_BPC_C"))
  (`/Engine/EditorBlueprintResources/StandardMacros.IsValid` _returnvalue
    (:`Is Valid`
      (`/Game/Game/Blueprints/Component/Actor/BETA_MainHUDComponent_BPC.OnEnterHiddenObjectRange` _returnvalue self))))

(event `self.HighlightRange.OnComponentEndOverlap`
  (params (OverlappedComponent :type "PrimitiveComponent Object Reference") (OtherActor :type "Actor Object Reference") (OtherComp :type "PrimitiveComponent Object Reference") (OtherBodyIndex :type Integer))
  (bind _returnvalue (`self.GetComponentByClass` OtherActor "/Game/Game/Blueprints/Component/Actor/BETA_MainHUDComponent_BPC.BETA_MainHUDComponent_BPC_C"))
  (`/Engine/EditorBlueprintResources/StandardMacros.IsValid` _returnvalue
    (:`Is Valid`
      (`/Game/Game/Blueprints/Component/Actor/BETA_MainHUDComponent_BPC.OnLeaveHiddenObjectRange` _returnvalue self))))

(fn `UserConstructionScript`
  (`SphereComponent.SetSphereRadius` (`self.HighlightRange`) (`self.HighlightRadius`) true))