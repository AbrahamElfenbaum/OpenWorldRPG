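; Master Blueprint for map landmarks, such as towers and towns, that become discovered when approached.
; The construction script picks the billboard sprite from the landmark Type and sizes the DiscoverArea sphere from DiscoverRadius.
; When an actor with an InGameHUD_BPC component overlaps the sphere, it sets IsDiscovered and destroys the sphere, so discovery happens only once.
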(event `self.DiscoverArea.OnComponentBeginOverlap`
  (params (OverlappedComponent :type "PrimitiveComponent Object Reference") (OtherActor :type "Actor Object Reference") (OtherComp :type "PrimitiveComponent Object Reference") (OtherBodyIndex :type Integer) (bFromSweep :type Boolean) (SweepResult :type "HitResult Structure (by ref)"))
  (`/Engine/EditorBlueprintResources/StandardMacros.IsValid` (`self.GetComponentByClass` OtherActor "/Game/Game/Blueprints/Components/Actors/InGameHUD_BPC.InGameHUD_BPC_C")
    (:`Is Valid`
      (set `self.isDiscovered` true)
      (`ActorComponent.K2_DestroyComponent` (`self.DiscoverArea`)))))

(fn `UserConstructionScript`
  (`BillboardComponent.SetSprite` (`self.Billboard`) (select `/Game/Game/Blueprints/Enums/LandmarkType_E` (`self.Type`) :`NewEnumerator0` "/Game/Game/Textures/UI/Landmark_Tower_T.Landmark_Tower_T" :`NewEnumerator1` "/Game/Game/Textures/UI/Landmark_Town_T.Landmark_Town_T" :!type "Texture2D Object Reference"))
  (`SphereComponent.SetSphereRadius` (`self.DiscoverArea`) (`self.DiscoverRadius`) false))