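; Master waypoint actor that players discover on the map by getting close to it.
; The construction script sizes a DiscoverRange sphere from DiscoverRadius.
; When an overlapping actor has an InGameHUD_BPC component, the waypoint passes itself to that component's MapDiscoverWaypoint.
; An OnDiscover event destroys the sphere, removing the discovery trigger.
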(event `OnDiscover`
  (`ActorComponent.K2_DestroyComponent` (`self.DiscoverRange`)))

(event `self.DiscoverRange.OnComponentBeginOverlap`
  (params (OverlappedComponent :type "PrimitiveComponent Object Reference") (OtherActor :type "Actor Object Reference") (OtherComp :type "PrimitiveComponent Object Reference") (OtherBodyIndex :type Integer) (bFromSweep :type Boolean) (SweepResult :type "HitResult Structure (by ref)"))
  (bind _returnvalue (`self.GetComponentByClass` OtherActor "/Game/Game/Blueprints/Components/Actors/InGameHUD_BPC.InGameHUD_BPC_C"))
  (`/Engine/EditorBlueprintResources/StandardMacros.IsValid` _returnvalue
    (:`Is Valid`
      (`/Game/Game/Blueprints/Components/Actors/InGameHUD_BPC.MapDiscoverWaypoint` _returnvalue self))))

(fn `UserConstructionScript`
  (`SphereComponent.SetSphereRadius` (`self.DiscoverRange`) (`self.DiscoverRadius`) false))